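; Animal character Blueprint that plays a particle effect and flags its AnimalController for Kill when the animal is in the Spawn or Exit state.
; BeginPlay caches the AnimalController, and Tick polls its current state.
; On a match, Tick spawns the effect at the actor's location and sets the state to Kill.
; An unconnected branch that would set walk speed never runs.
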(event EventBeginPlay
  (bind _asanimal_controller (Utilities|Casting|CastToAnimalController (Pawn|GetController))))

(event Collision|EventActorBeginOverlap
  (params (OtherActor :type Actor%20Object%20Reference)))

(event EventTick
  (params (DeltaSeconds :type Float%20%28single-precision%29))
  (if (Math|Boolean|ORBoolean (Utilities|Enum|Equal(Enum) (Variables|/Script/TeamWolverineProject.AnimalController|GetmCurrentState (stale EventBeginPlay _asanimal_controller)) "Spawn") (Utilities|Enum|Equal(Enum) (Variables|/Script/TeamWolverineProject.AnimalController|GetmCurrentState (stale EventBeginPlay _asanimal_controller)) "Exit") false)
    (Effects|SpawnEmitteratLocation (Variables|Default|GetmParticleEffect) (Math|Transform|TransformLocation (Transformation|GetActorTransform) "0, 0, 0"))
    (if true
      (Variables|/Script/TeamWolverineProject.AnimalController|SetmCurrentState (stale EventBeginPlay _asanimal_controller) "Kill"))))

(fn ConstructionScript)