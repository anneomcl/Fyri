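; BP_GameManager is the actor that routes player input to an ObjectManager for choosing and spawning objects.
; On BeginPlay it enables player input and initializes the ObjectManager with every BP_Tile actor in the level.
; Three button click events set the manager's current object by index, and releasing the left mouse button tells it to spawn an object.
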(event OnClicked(Button_205)
  (Class|ObjectManagerComponent|UpdateCurrentObject (Variables|Default|GetObjectManager)))

(event OnClicked(Button_206)
  (Class|ObjectManagerComponent|UpdateCurrentObject (Variables|Default|GetObjectManager) 1))

(event OnClicked(Button_207)
  (Class|ObjectManagerComponent|UpdateCurrentObject (Variables|Default|GetObjectManager) 2))

(event EventBeginPlay
  (Input|EnableInput (Game|GetPlayerController 0))
  (bind _outactors (Actor|GetAllActorsOfClass "/Game/Blueprints/BP_Tile.BP_Tile_C"))
  (Class|ObjectManagerComponent|Init (Variables|Default|GetObjectManager) _outactors))

(event Collision|EventActorBeginOverlap
  (params (OtherActor :type Actor%20Object%20Reference)))

(event EventTick
  (params (DeltaSeconds :type Float%20%28single-precision%29)))

(event Input|MouseEvents|LeftMouseButton
  (params (Key :type Key%20Structure))
  (:Released
    (Class|ObjectManagerComponent|SpawnObject (Variables|Default|GetObjectManager))))

(fn ConstructionScript)