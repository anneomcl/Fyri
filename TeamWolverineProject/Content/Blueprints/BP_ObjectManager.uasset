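; Object manager for a tile-based planting game that spawns objects and handles feedback when they spawn or interact.
; On BeginPlay it enables input and initializes with all grass middle tiles; releasing left mouse calls SpawnObject, and spawns play an explosion sound.
; Interactions play the result's particle and sound, then change Plant spawn probability once the "PlantWithTree" quantity is met.
; The interaction animation override is an unimplemented TODO.
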(event EventBeginPlay
  (Input|EnableInput (Game|GetPlayerController 0))
  (bind _outactors (Actor|GetAllActorsOfClass "/Game/Blueprints/Tiles/BP_GrassTileMiddle.BP_GrassTileMiddle_C"))
  (Class|ObjectManagerComponent|Init _outactors))

(event Collision|EventActorBeginOverlap
  (params (OtherActor :type Actor%20Object%20Reference)))

(event EventTick
  (params (DeltaSeconds :type Float%20%28single-precision%29)))

(event EventOnInteractionStart
  (params (interactionResult :type Interaction%20Result%20Object%20Reference) (interactionLocation :type Vector%20%28by%20ref%29 :default "0, 0, 0"))
  (bind _mparticleeffect (Variables|/Script/TeamWolverineProject.InteractionResult|GetmParticleEffect interactionResult))
  (bind _msound (Variables|/Script/TeamWolverineProject.InteractionResult|GetmSound interactionResult))
  (Utilities|FlowControl|Sequence
    (:then_0
      ;[1 1 1] Interaction particle effect
      (Utilities|IsValid _mparticleeffect
        (:Is%20Valid
          (Effects|SpawnEmitteratLocation _mparticleeffect interactionLocation))))
    (:then_1
      ;[1 1 1] Play interaction sound. TODO: is currently looping??
      (Utilities|IsValid _msound
        (:Is%20Valid
          (Audio|PlaySoundatLocation _msound "0, 0, 0" "0, 0, 0" 1.0 1.0 0.0 0 0 0))))
    (:then_2
      ;[1 1 1] TODO ANIM: override animation with interaction anim
      (Utilities|IsValid (Variables|/Script/TeamWolverineProject.InteractionResult|GetmAnimation interactionResult)))
    (:then_3
      (if (Class|ObjectManagerComponent|HasPlantedRequiredQuantityOfObject "PlantWithTree")
        (Class|ObjectManagerComponent|ChangeSpawnProbability "Plant")))))

(event EventOnObjectSpawned
  (params (spawnedObject :type Plantable%20Object%20Object%20Reference))
  (Audio|PlaySoundatLocation "/Game/StarterContent/Audio/Explosion02.Explosion02" (Transformation|GetActorLocation spawnedObject) "0, 0, 0" 0.3 1.0 0.0 0 0 0))

(event Input|MouseEvents|LeftMouseButton
  (params (Key :type Key%20Structure))
  (:Released
    (Class|ObjectManagerComponent|SpawnObject)))

(fn ConstructionScript)