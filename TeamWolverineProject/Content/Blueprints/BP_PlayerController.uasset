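; Player controller that gates input behind the game title screen, handles pausing, and relays plantable object selection.
; On BeginPlay it disables input in UI-only mode and binds to title widgets, restoring input in Game and UI mode when the title finishes.
; P opens a lazily created, cached pause menu, while UnpauseGame removes it and switches to game-only input.
; UpdateCurrentObject forwards the selected index to every BP_ObjectManager in the level.
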(event Custom|GameTitleFinished
  (bind _self self)
  (Input|EnableInput _self)
  (Input|SetInputModeGameandUI _self (Variables|Default|GetPauseMenu) "DoNotLock" false))

(event EventBeginPlay
  (Input|SetInputModeUIOnly self 0 "LockOnCapture")
  (Input|DisableInput self)
  (bind _foundwidgets (Widget|GetAllWidgetsOfClass "/Game/UI/GameTitleWidget.GameTitleWidget_C" true))
  (for _array_element _foundwidgets
    (EventDispatchers|BindEventtoGameTitleFinished _array_element (delegate Custom|GameTitleFinished))))

(event EventTick
  (params (DeltaSeconds :type Float%20%28single-precision%29)))

(event Input|KeyboardEvents|P
  (params (Key :type Key%20Structure))
  ;[1 1 1] Pause the game
  (:Pressed
    (CallFunction|PauseGame)))

(fn ConstructionScript)

(fn UpdateCurrentObject
  (params (ObjectIndex :type EPlantableObjectType%20Enum :default "Plant"))
  (bind _outactors (Actor|GetAllActorsOfClass "/Game/Blueprints/BP_ObjectManager.BP_ObjectManager_C"))
  (for _array_element _outactors
    (Class|ObjectManagerComponent|UpdateCurrentlySelectedPlantableObject _array_element ObjectIndex)))

(fn PauseGame
  (Game|SetGamePaused true)
  (Utilities|IsValid (Variables|Default|GetPauseMenu)
    (:Is%20Valid
      _)
    (:Is%20Not%20Valid
      (bind _returnvalue (UserInterface|CreateWidget "/Game/UI/UI_PauseMenu.UI_PauseMenu_C" (Game|GetPlayerController 0)))
      (Variables|Default|SetPauseMenu _returnvalue)))
  (UserInterface|Viewport|AddtoViewport (Variables|Default|GetPauseMenu) 0)
  (Input|SetInputModeUIOnly (Game|GetPlayerController 0) (Variables|Default|GetPauseMenu) "DoNotLock")
  (Variables|/Script/Engine.PlayerController|SetbShowMouseCursor (Game|GetPlayerController 0) true))

(fn UnpauseGame
  (bind _returnvalue (Game|GetPlayerController 0))
  (Game|SetGamePaused false)
  (Widget|RemovefromParent (Variables|Default|GetPauseMenu))
  (Input|SetInputModeGameOnly _returnvalue)
  (Variables|/Script/Engine.PlayerController|SetbShowMouseCursor _returnvalue true))