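; BP_CameraControls is a pawn that provides orbit and zoom controls for a boom-arm camera.
; Holding the right mouse button opens a gate that lets mouse X drive controller yaw.
; The mouse wheel steps the arm length within clamped limits and sets the boom's vertical target offset from that length, so height follows zoom.
; The camera-manager pitch limits and the alternative RightMouseButton boom-rotation function are disconnected and never run.
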(event EventBeginPlay
  ;[1 0.06771 0.06771] Limit Camera Pitch
)

(event Input|MouseEvents|MouseX
  (params (AxisValue :type Float%20%28single-precision%29))
  (bind _returnvalue (Pawn|GetControlRotation :!class /Script/Engine.Pawn))
  ;[0.2602 1 0.6012] Orbital Camera
  (Utilities|FlowControl|Gate true
    (:Exit
      (Pawn|Input|AddControllerYawInput AxisValue)
      (Pawn|SetControlRotation (Game|GetPlayerController 0) (Math|Rotator|MakeRotator 0.0 (.pitch _returnvalue) (.yaw _returnvalue))))))

(event Input|MouseEvents|MouseWheelDown
  (params (Key :type Key%20Structure))
  (bind _boomarm (Variables|Default|GetBoomArm))
  ;[0.2334 1 0.4532] Zoom In/Out
  (:Pressed
    (Variables|/Script/Engine.SpringArmComponent|SetTargetArmLength _boomarm (Math|Float|Clamp(Float) (+ (Variables|/Script/Engine.SpringArmComponent|GetTargetArmLength _boomarm) 1e+02) 5e+02 3e+03))
    (Variables|/Script/Engine.SpringArmComponent|SetTargetOffset _boomarm (Math|Vector|MakeVector 0.0 0.0 (Math|Float|Clamp(Float) (+ (Variables|/Script/Engine.SpringArmComponent|GetTargetArmLength _boomarm) 1e+02) 5e+02 3e+03)))))

(event Input|MouseEvents|RightMouseButton
  (params (Key :type Key%20Structure))
  (bind _returnvalue (Pawn|GetControlRotation :!class /Script/Engine.Pawn))
  ;[0.2602 1 0.6012] Orbital Camera
  (:Pressed
    (Utilities|FlowControl|Gate true) ; enters at Open
  )
  (:Released
    (Utilities|FlowControl|Gate true) ; enters at Close
  ))

(event Input|MouseEvents|MouseWheelUp
  (params (Key :type Key%20Structure))
  (bind _boomarm (Variables|Default|GetBoomArm))
  ;[0.2334 1 0.4532] Zoom In/Out
  (:Pressed
    (Variables|/Script/Engine.SpringArmComponent|SetTargetArmLength _boomarm (Math|Float|Clamp(Float) (- (Variables|/Script/Engine.SpringArmComponent|GetTargetArmLength _boomarm) 1e+02) 5e+02 3e+03))
    (Variables|/Script/Engine.SpringArmComponent|SetTargetOffset _boomarm (Math|Vector|MakeVector 0.0 0.0 (Math|Float|Clamp(Float) (- (Variables|/Script/Engine.SpringArmComponent|GetTargetArmLength _boomarm) 1e+02) 5e+02 3e+03)))))

(fn ConstructionScript)

(fn RightMouseButton
  (bind _boomarm (Variables|Default|GetBoomArm))
  (bind _returnvalue (Transformation|GetSocketTransform _boomarm "None" "RTS_World"))
  (bind _rotation (Math|Transform|BreakTransform _returnvalue))
  (bind (_roll _pitch _yaw) (Math|Rotator|BreakRotator _rotation))
  (Transformation|SetRelativeRotation _boomarm (Math|Rotator|MakeRotator 0.0 (Math|Float|Clamp(Float) (+ _pitch (* (Class|Actor|GetInputAxisKeyValue) 2.0)) -75.0) (+ _yaw (* (Class|Actor|GetInputAxisKeyValue) 2.0))) false false))